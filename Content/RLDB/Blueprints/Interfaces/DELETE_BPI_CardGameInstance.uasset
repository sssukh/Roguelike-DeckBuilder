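; Blueprint interface for a card game's Game Instance, apparently marked for deletion by its DELETE prefix, exposing persistent run state to other Blueprints.
; It declares accessors for the deck, artifacts, persistent heroes and their health, node map progress, current and completed story encounters, and reward settings.
; It also declares calls for saving, loading, resetting, debug mode and global graphics quality.
; All functions are signatures only, returning default values.
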(fn GetDeckfromInstance
  (return false 0))

(fn UpdateDeckinInstance
  (params (Cards :type Array%20of%20BP%20Card%20Object%20References)))

(fn ResetGame)

(fn GetArtifactsfromInstance
  (return 0))

(fn AddArtifacttoInstance
  (params (Artifact :type F%20Status%20Structure))
  (return false))

(fn GetMainHero
  (return false 0))

(fn IsDebugMode
  (return false))

(fn AttemptSaveGame
  (params (LevelNameOverride :type String) (bUpdateDeck :type Boolean))
  (return false))

(fn AttemptLoadGame
  (params (SaveIdIn :type String) (bOpenLevelIfValid :type Boolean))
  (return false))

(fn GetPlayerHero
  (return false 0))

(fn UpdateHeroPersistentHealth
  (params (HeroUniqueId :type String) (NewHealth :type Integer))
  (return false))

(fn GetGlobalGraphicsQuality
  (return 0))

(fn SetGlobalGraphicsQuality
  (params (Quality :type Integer)))

(fn GetInstanceSaveId
  (return ""))

(fn GetCurrentNodeMapfromInstance
  (return ""))

(fn GetVisitedMapNodesfromInstance
  (return 0))

(fn GetPersistentHeroesfromInstance
  (return 0))

(fn SetCurrentEncounterinInstance
  (params (CurrentEncounter :type F%20Encounter%20Structure)))

(fn GetCurrentEncounterfromInstance
  (return ""))

(fn AddVisitedNodetoInstance
  (params (NodeId :type Integer)))

(fn AddPersistentHerotoInstance
  (params (HeroData :type Data%20Table%20Row%20Handle%20Structure) (HeroDeck :type Data%20Table%20Row%20Handle%20Structure))
  (return false ""))

(fn RemovePersistentHerofromInstance
  (params (HeroUniqueId :type String))
  (return false))

(fn GetHerowithIdfromInstance
  (params (UniqueId :type String))
  (return false "" 0))

(fn SetRewardTables
  (params (RewardTables :type Array%20of%20Data%20Table%20Object%20References))
  (return false))

(fn GetRewardTables
  (return 0))

(fn GetDoneStoryEncountersfromInstance
  (return 0))

(fn AddDoneStoryEncountertoInstance
  (params (StoryEncounter :type Data%20Table%20Row%20Handle%20Structure)))

(fn CheckifInstanceHasArtifact
  (params (Artifact :type BP%20Status%20Class%20Reference))
  (return false))

(fn SetAllowedCardRewardsinInstance
  (params (AllowedCardRewards :type Gameplay%20Tag%20Container%20Structure)))

(fn GetAllowedCardRewardsfromInstance
  (return ""))

(fn ChangeNodeMapinInstance
  (params (NewNodeMap :type String))
  (return))