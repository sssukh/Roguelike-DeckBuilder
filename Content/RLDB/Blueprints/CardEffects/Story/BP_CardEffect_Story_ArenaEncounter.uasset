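; Card effect Blueprint for story cards that launches an arena encounter when resolved.
; It looks up the encounter row from the card's configured data table and row name.
; On success it saves the game with a deck update, stores the row as the game instance's current encounter, then opens that row's level.
; It returns false when the row is missing.
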(fn ResolveCardEffect
  (params (TargetActor :type Actor%20Object%20Reference))
  (bind _useddata (Variables|Default|GetUsedData))
  (bind _returnvalue (Utilities|GetDataTableRow (.datatable _useddata) (.rowname _useddata))
    (:then
      (Class|Object|AttemptSaveGame(Message) (Game|GetGameInstance) "" true)
      (Class|Object|SetCurrentEncounterinInstance(Message) (Game|GetGameInstance) _returnvalue)
      (Game|OpenLevel(byName) (Utilities|String|StringToName (.Level (Utilities|Struct|BreakFEncounter _returnvalue))))
      (return true))
    (:RowNotFound
      (return false))))