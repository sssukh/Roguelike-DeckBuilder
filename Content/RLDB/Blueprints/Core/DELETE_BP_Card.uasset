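; Card Blueprint for a deck-building game, holding one card's data; its DELETE_ name prefix suggests it is slated for removal.
; Keeps Base, Deck, Pile and Hand copies of the card struct, seeded from a data table or preset Deck data, so Hand changes can reset to Pile.
; Tag-filtered functions edit effect values, effects spawn as action actors, and card events route through a dispatcher hub.
; Playability, targeting and use functions are empty stubs.
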(fn ConstructionScript)

(fn CheckifPlayable)

(fn InitializefromData
  (bind _returnvalue (Components|GetOwner))
  (bind _datarowhandle (CardData|GetCardDataRowHandle "NewEnumerator1"))
  (bind _cardname (CardData|GetCardName "NewEnumerator1"))
  (bind _returnvalue_2 (Utilities|Text|TextIsEmpty _cardname))
  (if (Utilities|IsValid (.datatable _datarowhandle))
    (bind _returnvalue_3 (Utilities|GetDataTableRow (.datatable _datarowhandle) (.rowname _datarowhandle))
      (:then
        (Variables|Default|SetCardDataBase _returnvalue_3)
        (if _returnvalue_2
          (Variables|Default|SetCardDataDeck (Variables|Default|GetCardDataBase))))
      (:RowNotFound
        (if (not _returnvalue_2) :!label _label
          (Variables|Default|SetCardDataBase (Variables|Default|GetCardDataDeck))
          (else
            (Development|PrintString (Utilities|String|Append "ERROR: Attempted to initialize invalid card from data table (" (Utilities|GetDisplayName (.datatable _datarowhandle)) ") with name (" (Utilities|String|ToString(Name) (.rowname _datarowhandle)) ")"))
            (return)))))
    (else
      (goto _label)))
  (if (Utilities|IsValid _returnvalue)
    (bind _uniqueid (Class|BPICardTarget|GetMinionUniqueId(Message) _returnvalue))
    (Utilities|Struct|SetmembersinFCard (Variables|Default|GetCardDataDeck) _uniqueid))
  (bind _output_get (Variables|Default|SetCardDataPile (Variables|Default|GetCardDataDeck)))
  (Variables|Default|SetCardDataHand _output_get)
  (Variables|/Game/RLDB/Blueprints/Core/BP_GameplayTagComponent.BP_GameplayTagComponent_C|SetGameplayTags (Variables|Default|GetBP_GameplayTag_Component) (CardData|GetCardTags "NewEnumerator0")))

(fn FindAllPotentialTargets)

(fn ResolveUseRuleConsequences)

(fn Discard
  (params (CallTags :type Gameplay%20Tag%20Container%20Structure))
  (Default|CallEventwithCallTags (Variables|Default|GetBP_DispatcherHubComponent_Local) "(TagName=\"Event.Card.Discard\")" self 0 "NewEnumerator2" CallTags)
  (return))

(fn QueueCardEffectAction
  (params (TargetActor :type Actor%20Object%20Reference) (SourcePuppet :type Actor%20Object%20Reference) (CardEffect :type BP%20Card%20Effect%20Object%20Reference) (bAnimateSourcePuppet :type Boolean))
  (bind _effectaction (Variables|/Game/RLDB/Blueprints/CardEffects/BP_CardEffect.BP_CardEffect_C|GetEffectAction CardEffect))
  (if (Utilities|IsValidClass _effectaction)
    (Game|SpawnActorfromClass _effectaction (Math|Transform|MakeTransform "0, 0, 0" "0, 0, 0" "1.000000,1.000000,1.000000") "Undefined" "SelectDefaultAtRuntime" 0 TargetActor SourcePuppet (select bAnimateSourcePuppet (Variables|/Game/RLDB/Blueprints/CardEffects/BP_CardEffect.BP_CardEffect_C|GetHeroAnim CardEffect) "") (Utilities|Array|Get(acopy) (CardData|GetCardEffects "NewEnumerator0") (Variables|Default|GetEffectLoopIndex)) -1.0 0)
    (return)
    (else
      (return))))

(fn Exhaust
  (Default|CallEvent (Variables|Default|GetBP_DispatcherHubComponent_Local) "(TagName=\"Event.Card.Exhaust\")" self 0 "NewEnumerator2")
  (return))

(fn GetGameplayTags
  (return (Variables|/Game/RLDB/Blueprints/Core/BP_GameplayTagComponent.BP_GameplayTagComponent_C|GetGameplayTags (Variables|Default|GetBP_GameplayTag_Component))))

(fn AccessTargetingClassLazy
  (params (TargetingHolderActor :type Actor%20Object%20Reference) (TargetingClass :type BP%20Targeting%20Class%20Reference)))

(fn GetCardName
  (params (Type :type ECardDataType%20Enum :default "NewEnumerator0"))
  (return (Utilities|Struct|BreakFCard (Utilities|Select :Index Type :NewEnumerator0 (Variables|Default|GetCardDataHand) :NewEnumerator1 (Variables|Default|GetCardDataDeck) :NewEnumerator2 (Variables|Default|GetCardDataBase) :NewEnumerator3 (Variables|Default|GetCardDataPile)))))

(fn GetCardDescription
  (params (Type :type ECardDataType%20Enum :default "NewEnumerator0"))
  (return (Utilities|Struct|BreakFCard (Utilities|Select :Index Type :NewEnumerator0 (Variables|Default|GetCardDataHand) :NewEnumerator1 (Variables|Default|GetCardDataDeck) :NewEnumerator2 (Variables|Default|GetCardDataBase) :NewEnumerator3 (Variables|Default|GetCardDataPile)))))

(fn GetCardPortrait
  (params (Type :type ECardDataType%20Enum :default "NewEnumerator0"))
  (return (Utilities|Struct|BreakFCard (Utilities|Select :Index Type :NewEnumerator0 (Variables|Default|GetCardDataHand) :NewEnumerator1 (Variables|Default|GetCardDataDeck) :NewEnumerator2 (Variables|Default|GetCardDataBase) :NewEnumerator3 (Variables|Default|GetCardDataPile)))))

(fn GetCardTooltips
  (params (Type :type ECardDataType%20Enum :default "NewEnumerator0"))
  (return (Utilities|Struct|BreakFCard (Utilities|Select :Index Type :NewEnumerator0 (Variables|Default|GetCardDataHand) :NewEnumerator1 (Variables|Default|GetCardDataDeck) :NewEnumerator2 (Variables|Default|GetCardDataBase) :NewEnumerator3 (Variables|Default|GetCardDataPile)))))

(fn GetCardTags
  (params (Type :type ECardDataType%20Enum :default "NewEnumerator0"))
  (return (Utilities|Struct|BreakFCard (Utilities|Select :Index Type :NewEnumerator0 (Variables|Default|GetCardDataHand) :NewEnumerator1 (Variables|Default|GetCardDataDeck) :NewEnumerator2 (Variables|Default|GetCardDataBase) :NewEnumerator3 (Variables|Default|GetCardDataPile)))))

(fn GetCardTargeted
  (params (Type :type ECardDataType%20Enum :default "NewEnumerator0"))
  (return (Utilities|Struct|BreakFCard (Utilities|Select :Index Type :NewEnumerator0 (Variables|Default|GetCardDataHand) :NewEnumerator1 (Variables|Default|GetCardDataDeck) :NewEnumerator2 (Variables|Default|GetCardDataBase) :NewEnumerator3 (Variables|Default|GetCardDataPile)))))

(fn GetCardEffects
  (params (Type :type ECardDataType%20Enum :default "NewEnumerator0"))
  (return (Utilities|Struct|BreakFCard (Utilities|Select :Index Type :NewEnumerator0 (Variables|Default|GetCardDataHand) :NewEnumerator1 (Variables|Default|GetCardDataDeck) :NewEnumerator2 (Variables|Default|GetCardDataBase) :NewEnumerator3 (Variables|Default|GetCardDataPile)))))

(fn GetCardUseRules
  (params (Type :type ECardDataType%20Enum :default "NewEnumerator0")))

(fn GetCardStartingStatuses
  (params (Type :type ECardDataType%20Enum :default "NewEnumerator0")))

(fn GetCardFrame
  (params (Type :type ECardDataType%20Enum :default "NewEnumerator0"))
  (return (Utilities|Struct|BreakFCard (Utilities|Select :Index Type :NewEnumerator0 (Variables|Default|GetCardDataHand) :NewEnumerator1 (Variables|Default|GetCardDataDeck) :NewEnumerator2 (Variables|Default|GetCardDataBase) :NewEnumerator3 (Variables|Default|GetCardDataPile)))))

(fn GetCardDataRowHandle
  (params (Type :type ECardDataType%20Enum :default "NewEnumerator0"))
  (return (Utilities|Struct|BreakFCard (Utilities|Select :Index Type :NewEnumerator0 (Variables|Default|GetCardDataHand) :NewEnumerator1 (Variables|Default|GetCardDataDeck) :NewEnumerator2 (Variables|Default|GetCardDataBase) :NewEnumerator3 (Variables|Default|GetCardDataPile)))))

(fn GetCardFrameTint
  (params (Type :type ECardDataType%20Enum :default "NewEnumerator0"))
  (return (Utilities|Struct|BreakFCard (Utilities|Select :Index Type :NewEnumerator0 (Variables|Default|GetCardDataHand) :NewEnumerator1 (Variables|Default|GetCardDataDeck) :NewEnumerator2 (Variables|Default|GetCardDataBase) :NewEnumerator3 (Variables|Default|GetCardDataPile)))))

(fn GetCardOwnerID
  (params (Type :type ECardDataType%20Enum :default "NewEnumerator0"))
  (return (Utilities|Struct|BreakFCard (Utilities|Select :Index Type :NewEnumerator0 (Variables|Default|GetCardDataHand) :NewEnumerator1 (Variables|Default|GetCardDataDeck) :NewEnumerator2 (Variables|Default|GetCardDataBase) :NewEnumerator3 (Variables|Default|GetCardDataPile)))))

(fn GetCardVisualWidget
  (params (Type :type ECardDataType%20Enum :default "NewEnumerator0"))
  (return (Utilities|Struct|BreakFCard (Utilities|Select :Index Type :NewEnumerator0 (Variables|Default|GetCardDataHand) :NewEnumerator1 (Variables|Default|GetCardDataDeck) :NewEnumerator2 (Variables|Default|GetCardDataBase) :NewEnumerator3 (Variables|Default|GetCardDataPile)))))

(fn GetPostUseEvent
  (params (Type :type ECardDataType%20Enum :default "NewEnumerator0"))
  (return (Utilities|Struct|BreakFCard (Utilities|Select :Index Type :NewEnumerator0 (Variables|Default|GetCardDataHand) :NewEnumerator1 (Variables|Default|GetCardDataDeck) :NewEnumerator2 (Variables|Default|GetCardDataBase) :NewEnumerator3 (Variables|Default|GetCardDataPile)))))

(fn GetCardRepetitions
  (params (Type :type ECardDataType%20Enum :default "NewEnumerator0"))
  (return (Utilities|Struct|BreakFCard (Utilities|Select :Index Type :NewEnumerator0 (Variables|Default|GetCardDataHand) :NewEnumerator1 (Variables|Default|GetCardDataDeck) :NewEnumerator2 (Variables|Default|GetCardDataBase) :NewEnumerator3 (Variables|Default|GetCardDataPile)))))

(fn GetCardEndTurnEvent
  (params (Type :type ECardDataType%20Enum :default "NewEnumerator0"))
  (return (Utilities|Struct|BreakFCard (Utilities|Select :Index Type :NewEnumerator0 (Variables|Default|GetCardDataHand) :NewEnumerator1 (Variables|Default|GetCardDataDeck) :NewEnumerator2 (Variables|Default|GetCardDataBase) :NewEnumerator3 (Variables|Default|GetCardDataPile)))))

(fn SetCardName
  (params (Type :type ECardDataType%20Enum :default "NewEnumerator0") (CardName :type Text))
  (Utilities|Struct|SetmembersinFCard (Utilities|Select :Index Type :NewEnumerator0 (Variables|Default|GetCardDataHand) :NewEnumerator1 (Variables|Default|GetCardDataDeck) :NewEnumerator2 (Variables|Default|GetCardDataBase) :NewEnumerator3 (Variables|Default|GetCardDataPile)) CardName)
  (return))

(fn SetCardDescription
  (params (Type :type ECardDataType%20Enum :default "NewEnumerator0") (Description :type Text))
  (Utilities|Struct|SetmembersinFCard (Utilities|Select :Index Type :NewEnumerator0 (Variables|Default|GetCardDataHand) :NewEnumerator1 (Variables|Default|GetCardDataDeck) :NewEnumerator2 (Variables|Default|GetCardDataBase) :NewEnumerator3 (Variables|Default|GetCardDataPile)) Description)
  (return))

(fn SetCardPortrait
  (params (Type :type ECardDataType%20Enum :default "NewEnumerator0") (Portrait :type Texture%202D%20Object%20Reference))
  (Utilities|Struct|SetmembersinFCard (Utilities|Select :Index Type :NewEnumerator0 (Variables|Default|GetCardDataHand) :NewEnumerator1 (Variables|Default|GetCardDataDeck) :NewEnumerator2 (Variables|Default|GetCardDataBase) :NewEnumerator3 (Variables|Default|GetCardDataPile)) Portrait)
  (return))

(fn SetCardTooltips
  (params (Type :type ECardDataType%20Enum :default "NewEnumerator0") (Tooltips :type Array%20of%20Data%20Table%20Row%20Handle%20Structures))
  (Utilities|Struct|SetmembersinFCard (Utilities|Select :Index Type :NewEnumerator0 (Variables|Default|GetCardDataHand) :NewEnumerator1 (Variables|Default|GetCardDataDeck) :NewEnumerator2 (Variables|Default|GetCardDataBase) :NewEnumerator3 (Variables|Default|GetCardDataPile)) Tooltips)
  (return))

(fn SetCardCardTags
  (params (Type :type ECardDataType%20Enum :default "NewEnumerator0") (CardTags :type Gameplay%20Tag%20Container%20Structure))
  (Utilities|Struct|SetmembersinFCard (Utilities|Select :Index Type :NewEnumerator0 (Variables|Default|GetCardDataHand) :NewEnumerator1 (Variables|Default|GetCardDataDeck) :NewEnumerator2 (Variables|Default|GetCardDataBase) :NewEnumerator3 (Variables|Default|GetCardDataPile)) CardTags)
  (return))

(fn SetCardTargeted
  (params (Type :type ECardDataType%20Enum :default "NewEnumerator0") (bTargeted :type Boolean))
  (Utilities|Struct|SetmembersinFCard (Utilities|Select :Index Type :NewEnumerator0 (Variables|Default|GetCardDataHand) :NewEnumerator1 (Variables|Default|GetCardDataDeck) :NewEnumerator2 (Variables|Default|GetCardDataBase) :NewEnumerator3 (Variables|Default|GetCardDataPile)) bTargeted)
  (return))

(fn SetCardEffects
  (params (Type :type ECardDataType%20Enum :default "NewEnumerator0") (CardEffects :type Array%20of%20F%20Card%20Effect%20Structures))
  (Utilities|Struct|SetmembersinFCard (Utilities|Select :Index Type :NewEnumerator0 (Variables|Default|GetCardDataHand) :NewEnumerator1 (Variables|Default|GetCardDataDeck) :NewEnumerator2 (Variables|Default|GetCardDataBase) :NewEnumerator3 (Variables|Default|GetCardDataPile)) CardEffects)
  (return))

(fn SetCardFrame
  (params (Type :type ECardDataType%20Enum :default "NewEnumerator0") (Frame :type Texture%202D%20Object%20Reference))
  (Utilities|Struct|SetmembersinFCard (Utilities|Select :Index Type :NewEnumerator0 (Variables|Default|GetCardDataHand) :NewEnumerator1 (Variables|Default|GetCardDataDeck) :NewEnumerator2 (Variables|Default|GetCardDataBase) :NewEnumerator3 (Variables|Default|GetCardDataPile)) Frame)
  (return))

(fn SetCardFrameTint
  (params (Type :type ECardDataType%20Enum :default "NewEnumerator0") (FrameTint :type Slate%20Color%20Structure))
  (Utilities|Struct|SetmembersinFCard (Utilities|Select :Index Type :NewEnumerator0 (Variables|Default|GetCardDataHand) :NewEnumerator1 (Variables|Default|GetCardDataDeck) :NewEnumerator2 (Variables|Default|GetCardDataBase) :NewEnumerator3 (Variables|Default|GetCardDataPile)) FrameTint)
  (return))

(fn ResetinHandModifications
  (Variables|Default|SetCardDataHand (Variables|Default|GetCardDataPile))
  (return))

(fn SetCardOwnerID
  (params (Type :type ECardDataType%20Enum :default "NewEnumerator0") (OwnerID :type String))
  (Utilities|Struct|SetmembersinFCard (Utilities|Select :Index Type :NewEnumerator0 (Variables|Default|GetCardDataHand) :NewEnumerator1 (Variables|Default|GetCardDataDeck) :NewEnumerator2 (Variables|Default|GetCardDataBase) :NewEnumerator3 (Variables|Default|GetCardDataPile)) OwnerID)
  (return))

(fn AttemptUseCard
  (params (Targets :type Array%20of%20Actor%20Object%20References) (bSkipPlayableCheck :type Boolean) (bSkipConsequences :type Boolean) (bAutoPlay :type Boolean)))

(fn SetCardRarityfromTags
  (if (GameplayTags|HasTag (CardData|GetCardTags "NewEnumerator2") "(TagName=\"Rarity\")")
    (for _array_element (.gameplaytags (LocalVariables|GetLocalRarities))
      (if (GameplayTags|HasTag (CardData|GetCardTags "NewEnumerator2") _array_element true)
        (bind _output_get (Variables|Default|SetRarity _array_element))
        (return _output_get))))
  (bind _output_get_2 (Variables|Default|SetRarity "(TagName=\"Rarity.Invalid\")"))
  (return _output_get_2))

(fn SetCardVisualWidget
  (params (Type :type ECardDataType%20Enum :default "NewEnumerator0") (CardVisualWidget :type User%20Widget%20Class%20Reference))
  (Utilities|Struct|SetmembersinFCard (Utilities|Select :Index Type :NewEnumerator0 (Variables|Default|GetCardDataHand) :NewEnumerator1 (Variables|Default|GetCardDataDeck) :NewEnumerator2 (Variables|Default|GetCardDataBase) :NewEnumerator3 (Variables|Default|GetCardDataPile)) CardVisualWidget)
  (return))

(fn SetCardTypefromTags
  (for _array_element (.gameplaytags (LocalVariables|GetLocalTypes))
    (if (GameplayTags|HasTag (CardData|GetCardTags "NewEnumerator2") _array_element true)
      (bind _output_get (Variables|Default|SetType _array_element))
      (return _output_get)))
  (bind _output_get_2 (Variables|Default|SetType "(TagName=\"Effect.Invalid\")"))
  (return _output_get_2))

(fn SetPostUseEvent
  (params (Type :type ECardDataType%20Enum :default "NewEnumerator0") (PostUseEvent :type Gameplay%20Tag%20Structure))
  (Utilities|Struct|SetmembersinFCard (Utilities|Select :Index Type :NewEnumerator0 (Variables|Default|GetCardDataHand) :NewEnumerator1 (Variables|Default|GetCardDataDeck) :NewEnumerator2 (Variables|Default|GetCardDataBase) :NewEnumerator3 (Variables|Default|GetCardDataPile)) PostUseEvent)
  (return))

(fn SetCardRepetitions
  (params (Type :type ECardDataType%20Enum :default "NewEnumerator0") (Repetitions :type Integer))
  (Utilities|Struct|SetmembersinFCard (Utilities|Select :Index Type :NewEnumerator0 (Variables|Default|GetCardDataHand) :NewEnumerator1 (Variables|Default|GetCardDataDeck) :NewEnumerator2 (Variables|Default|GetCardDataBase) :NewEnumerator3 (Variables|Default|GetCardDataPile)) Repetitions)
  (return))

(fn ModifyCardEffectValues
  (params (Modification :type Integer) (Type :type ECardDataType%20Enum :default "NewEnumerator0") (PossibleTags :type Gameplay%20Tag%20Container%20Structure) (RequiredTags :type Gameplay%20Tag%20Container%20Structure))
  (LocalVariables|SetbLocalNoPossibleTags (== (GameplayTags|GetNumGameplayTagsinContainer PossibleTags) 0))
  (LocalVariables|SetbLocalNoRequiredTags (== (GameplayTags|GetNumGameplayTagsinContainer RequiredTags) 0))
  (bind _output_get (LocalVariables|SetLocalCardEffects (CardData|GetCardEffects Type)))
  (for (_array_element _array_index) _output_get
    (if (and (or (LocalVariables|GetbLocalNoPossibleTags) (GameplayTags|HasAnyTags (.GameplayTags (Utilities|Struct|BreakFCardEffect _array_element)) PossibleTags true)) (or (LocalVariables|GetbLocalNoRequiredTags) (GameplayTags|HasAllTags (.GameplayTags (Utilities|Struct|BreakFCardEffect _array_element)) RequiredTags true)))
      (LocalVariables|SetbLocalCardModified true)
      (Utilities|Struct|SetmembersinFCardEffect (Utilities|Array|Get(acopy) (LocalVariables|GetLocalCardEffects) _array_index) (Math|Integer|Max(Integer) (+ (.EffectValue (Utilities|Struct|BreakFCardEffect _array_element)) Modification)))))
  (if (LocalVariables|GetbLocalCardModified)
    (CardData|SetCardEffects Type (LocalVariables|GetLocalCardEffects))
    (Default|CallOnThisCardModified)
    (return)
    (else
      (return))))

(fn GetCardEffectValue
  (params (PossibleTags :type Gameplay%20Tag%20Container%20Structure) (RequiredTags :type Gameplay%20Tag%20Container%20Structure) (Type :type ECardDataType%20Enum :default "NewEnumerator0"))
  (bind _output_get (LocalVariables|SetLocalCardEffects (CardData|GetCardEffects Type)))
  (for _array_element _output_get
    (if (and (or (== (GameplayTags|GetNumGameplayTagsinContainer PossibleTags) 0) (GameplayTags|HasAnyTags (.GameplayTags (Utilities|Struct|BreakFCardEffect _array_element)) PossibleTags true)) (or (== (GameplayTags|GetNumGameplayTagsinContainer RequiredTags) 0) (GameplayTags|HasAllTags (.GameplayTags (Utilities|Struct|BreakFCardEffect _array_element)) RequiredTags true)))
      (return true (.EffectValue (Utilities|Struct|BreakFCardEffect _array_element)))))
  (return false 0))

(fn IsinHand
  (return (== (Variables|Default|GetCurrentPile) "(TagName=\"Pile.Hand\")")))

(fn AttemptUseCardUntargeted
  (params (bSkipPlayableCheck :type Boolean) (bSkipConsequences :type Boolean) (bAutoPlay :type Boolean)))

(fn GetStatusCostValuefromUseRules
  (params (Pile :type ECardDataType%20Enum :default "NewEnumerator0") (Status :type Object%20Class%20Reference)))

(fn SetUseRuleCost
  (params (UseRule :type BP%20Use%20Rule%20Stat%20Cost%20Class%20Reference) (Status :type BP%20Status%20Class%20Reference) (NewValue :type Integer) (Pile :type ECardDataType%20Enum :default "NewEnumerator0") (bAddIfNotFound :type Boolean)))

(fn CallLocalEventonCard
  (params (EventTag :type Gameplay%20Tag%20Structure) (AlsoCallGlobal :type ECallGlobal%20Enum :default "NewEnumerator2"))
  (bind _bsuccess (Default|CallEvent (Variables|Default|GetBP_DispatcherHubComponent_Local) EventTag self 0 AlsoCallGlobal))
  (return _bsuccess))

(fn RunEndTurnEvent
  (params (CallTags :type Gameplay%20Tag%20Container%20Structure))
  (bind _endturnevent (CardData|GetCardEndTurnEvent "NewEnumerator0"))
  (if (GameplayTags|IsGameplayTagValid _endturnevent)
    (Default|CallEventwithCallTags (Variables|Default|GetBP_DispatcherHubComponent_Local) _endturnevent self 0 "NewEnumerator2" CallTags)
    (return)
    (else
      (return))))

(fn SetCardEndTurnEvent
  (params (Type :type ECardDataType%20Enum :default "NewEnumerator0") (EndTurnEvent :type Gameplay%20Tag%20Structure))
  (Utilities|Struct|SetmembersinFCard (Utilities|Select :Index Type :NewEnumerator0 (Variables|Default|GetCardDataHand) :NewEnumerator1 (Variables|Default|GetCardDataDeck) :NewEnumerator2 (Variables|Default|GetCardDataBase) :NewEnumerator3 (Variables|Default|GetCardDataPile)) EndTurnEvent)
  (return))

(fn BindLocalCardEvents
  (params (EventHolder :type Object%20Object%20Reference) (EventTags :type Gameplay%20Tag%20Container%20Structure))
  (Default|BindMultipleEventstoHub (Variables|Default|GetBP_DispatcherHubComponent_Local) EventHolder EventTags)
  (return true))

(fn SetCardDatafromOtherData
  (params (From :type ECardDataType%20Enum :default "NewEnumerator0") (To :type ECardDataType%20Enum :default "NewEnumerator0"))
  (switch Utilities|FlowControl|Switch|SwitchonECardDataType To
    (:NewEnumerator0
      (Variables|Default|SetCardDataHand (Utilities|Select :Index From :NewEnumerator0 (Variables|Default|GetCardDataHand) :NewEnumerator1 (Variables|Default|GetCardDataDeck) :NewEnumerator2 (Variables|Default|GetCardDataBase) :NewEnumerator3 (Variables|Default|GetCardDataPile))))
    (:NewEnumerator1
      (Variables|Default|SetCardDataDeck (Utilities|Select :Index From :NewEnumerator0 (Variables|Default|GetCardDataHand) :NewEnumerator1 (Variables|Default|GetCardDataDeck) :NewEnumerator2 (Variables|Default|GetCardDataBase) :NewEnumerator3 (Variables|Default|GetCardDataPile))))
    (:NewEnumerator2
      (Variables|Default|SetCardDataBase (Utilities|Select :Index From :NewEnumerator0 (Variables|Default|GetCardDataHand) :NewEnumerator1 (Variables|Default|GetCardDataDeck) :NewEnumerator2 (Variables|Default|GetCardDataBase) :NewEnumerator3 (Variables|Default|GetCardDataPile))))
    (:NewEnumerator3
      (Variables|Default|SetCardDataPile (Utilities|Select :Index From :NewEnumerator0 (Variables|Default|GetCardDataHand) :NewEnumerator1 (Variables|Default|GetCardDataDeck) :NewEnumerator2 (Variables|Default|GetCardDataBase) :NewEnumerator3 (Variables|Default|GetCardDataPile)))))
  (return))