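; Minion track actor, prefixed DELETE, that holds an ordered Minions array with the first entry as front and the last as back.
; It returns either end with its index and computes centered slot positions along its box's local Y, with spacing shrinking as the count grows.
; Initiative is a modifier plus the minion's distance from the back, favoring the front.
; AddMinionToTrack is an empty stub.
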(fn ConstructionScript
  (|CallParentFunction))

(fn GetFrontMinion
  (bind _minions (Variables|Default|GetMinions))
  (bind _output (Utilities|Array|Get(acopy) _minions))
  (return (Utilities|IsValid _output) _output 0))

(fn GetBackMinion
  (bind _minions (Variables|Default|GetMinions))
  (bind _returnvalue (Utilities|Array|LastIndex _minions))
  (bind _output (Utilities|Array|Get(acopy) _minions _returnvalue))
  (return (Utilities|IsValid _output) _output _returnvalue))

(fn GetTrackLocationatIndex
  (params (TrackIndex :type Integer) (bNewSpawn :type Boolean))
  (bind _forwardoffset (Variables|Default|GetForwardOffset))
  (bind _minions (Variables|Default|GetMinions))
  (bind _returnvalue (Utilities|Array|LastIndex _minions))
  (bind _returnvalue_2 (+ _returnvalue bNewSpawn))
  (bind _returnvalue_3 (+ _returnvalue_2 _forwardoffset))
  (bind _returnvalue_4 (Math|Conversions|ToFloat(Integer) _returnvalue_3))
  (return (Math|Transform|TransformLocation (Transformation|GetActorTransform) (Math|Vector|MakeVector 0.0 (* (- (Math|Conversions|ToFloat(Integer) (+ TrackIndex (Variables|Default|GetForwardOffset))) (/ _returnvalue_4 2.0)) (* (* (* (/ 1.0 (+ _returnvalue_4 2.0)) (.y (Variables|/Script/Engine.BoxComponent|GetBoxExtent (Variables|Default|GetBox)))) -2.0) (.y (Transformation|GetActorScale3D)))) 0.0))))

(fn AddMiniontoTrack
  (params (Index :type Integer) (bSpawnedDuringGameplay :type Boolean)))

(fn GetInitiativefromTrack
  (params (Minion :type BP%20Minion%20Object%20Reference))
  (bind _minions (Variables|Default|GetMinions))
  (return (+ (Variables|Default|GetInitiativeModifier) (Math|Conversions|ToFloat(Integer) (Math|Integer|Max(Integer) (- (Utilities|Array|LastIndex _minions) (Utilities|Array|FindItem _minions Minion)))))))