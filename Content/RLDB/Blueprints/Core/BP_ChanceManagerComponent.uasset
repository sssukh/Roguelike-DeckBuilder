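; Component that serves random card picks by gameplay tag and rarity weights, apparently for rewards.
; Rarity and default-weight getters funnel into GetRandomCardsByTagWeights, designed around cumulative weighted tag rolls, shuffled duplicate-free matching, then random padding or a consolation card.
; That selection body and the DataTable loop filling AllCards on BeginPlay are disconnected, so neither runs.
; Artifact functions and the all-tags filter are empty stubs.
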(event EventBeginPlay
  (CallFunction|GenerateAllCardsArray)
  (CallFunction|GenerateAllArifactsArray))

(fn GetRandomCardsbyDefaultTagWeights
  (params (Amount :type Integer))
  (bind _randomcards (CallFunction|GetRandomCardsbyTagWeights :TagWeights (Variables|Default|GetDefaultCardTagWeights) :Amount Amount))
  (return _randomcards))

(fn GetRandomCardsOfSpecificRarity
  (params (Rarity :type Gameplay%20Tag%20Structure) (Amount :type Integer))
  (bind _randomcards (CallFunction|GetRandomCardsbyTagWeights :TagWeights (Utilities|Map|MakeMap Rarity 1.0) :Amount Amount))
  (return _randomcards))

(fn GetTrueRandomCardsOfAnyRarity
  (params (Amount :type Integer))
  (bind _randomcards (CallFunction|GetRandomFilteredCards :Amount Amount :RequiredTags "(GameplayTags=((TagName=\"Rarity\")))"))
  (if (> Amount 1)
    (for _index (range 0 (- Amount 1))
      (Utilities|Array|Add (LocalVariables|GetLocalPickedCards) (Utilities|Array|Get(acopy) _randomcards _index)))
    (return (LocalVariables|GetLocalPickedCards))
    (else
      (return (Utilities|Array|MakeArray (Utilities|Array|Get(acopy) _randomcards))))))

(fn GetRandomArtifactsbyCustomTagWeights
  (params (TagWeights :type Map%20of%20Gameplay%20Tag%20Structures%20to%20Reals) (Amount :type Integer) (bExactMatch :type Boolean)))

(fn GetRandomArtifactsbyDefaultRarityWeights
  (params (Amount :type Integer)))

(fn GetFilteredCardswithAnyTag
  (params (Filter :type Gameplay%20Tag%20Container%20Structure) (Cards :type Array%20of%20F%20Card%20Structures) (bExactMatch :type Boolean))
  (for _array_element Cards
    (if (GameplayTags|HasAnyTags (Utilities|Struct|BreakFCard _array_element) Filter bExactMatch)
      (Utilities|Array|Add (LocalVariables|GetLocalFilteredCards) _array_element)))
  (return (LocalVariables|GetLocalFilteredCards)))

(fn GetRandomCardsbyTagWeights
  (params (TagWeights :type Map%20of%20Gameplay%20Tag%20Structures%20to%20Reals) (PossibleTags :type Gameplay%20Tag%20Container%20Structure) (RequiredTags :type Gameplay%20Tag%20Container%20Structure) (bExactMatch :type Boolean) (Amount :type Integer))
  (LocalVariables|SetLocalFilteredCards (Variables|Default|GetAllCards)))

(fn FindPickedTagAmongFilteredCards
  (params (PickedCardTag :type Gameplay%20Tag%20Structure) (FilteredCards :type Array%20of%20F%20Card%20Structures) (bPreventDuplicates :type Boolean))
  (bind (_arrayindex _arrayelement) (Utilities|Array|ReverseforEachLoop FilteredCards)
    (:LoopBody
      (if (GameplayTags|HasTag (Utilities|Struct|BreakFCard _arrayelement) PickedCardTag true)
        (LocalVariables|SetLocalPickedCard _arrayelement)
        (if bPreventDuplicates
          (Utilities|Array|RemoveIndex FilteredCards _arrayindex))
        (return true (LocalVariables|GetLocalPickedCard))))
    (:Completed
      (return false ""))))

(fn GetCardsbyDefaultRarityWeights
  (params (Amount :type Integer))
  (bind _randomcards (CallFunction|GetRandomCardsbyTagWeights :TagWeights (Variables|Default|GetDefaultCardTagWeights) :Amount Amount))
  (return _randomcards))

(fn GenerateAllCardsArray
  (Utilities|Array|Clear (Variables|Default|GetAllCards)))

(fn GetRandomTagsbyWeights
  (params (WeightedTags :type Map%20of%20Gameplay%20Tag%20Structures%20to%20Reals) (Amount :type Integer))
  (bind _values (Utilities|Map|Values WeightedTags))
  (if (== (.MaxValue (Math|Float|MaxOfFloatArray _values)) (.MinValue (Math|Float|MinOfFloatArray _values))) ; If all weights are identical, simply pick random tags
    (while (< (Utilities|Array|Length (LocalVariables|GetLocalPickedTags)) Amount)
      (bind _keys (Utilities|Map|Keys WeightedTags))
      (Utilities|Array|Add (LocalVariables|GetLocalPickedTags) (.OutItem (Utilities|Array|Random _keys))))
    (return (LocalVariables|GetLocalPickedTags))
    (else
      (for _array_element _values
        (LocalVariables|SetLocalWeightSum (+ _array_element (LocalVariables|GetLocalWeightSum))))
      (while (< (Utilities|Array|Length (LocalVariables|GetLocalPickedTags)) Amount)
        (bind (_bsuccess _pickedtag) (CallFunction|PickTagfromWeightandWeightSum WeightedTags (LocalVariables|GetLocalWeightSum)))
        (if _bsuccess
          (Utilities|Array|Add (LocalVariables|GetLocalPickedTags) _pickedtag)))
      (return (LocalVariables|GetLocalPickedTags)))))

(fn PickTagfromWeightandWeightSum
  (params (WeightedTags :type Map%20of%20Gameplay%20Tag%20Structures%20to%20Reals) (WeightSum :type Float%20%28double-precision%29))
  (LocalVariables|SetLocalWeightSelection (Math|Random|RandomFloatinRange 0.0 WeightSum))
  (bind _keys (Utilities|Map|Keys WeightedTags))
  (for _array_element _keys
    (bind _output_get (LocalVariables|SetLocalWeightCount (+ (LocalVariables|GetLocalWeightCount) (.Value (Utilities|Map|Find WeightedTags _array_element)))))
    (if (>= _output_get (LocalVariables|GetLocalWeightSelection))
      (return true _array_element)))
  (return false ""))

(fn GenerateAllArifactsArray)

(fn GetFilteredCardswithAllTags
  (params (Filter :type Gameplay%20Tag%20Container%20Structure) (Cards :type Array%20of%20F%20Card%20Structures) (bExactMatch :type Boolean)))

(fn GetRemainingArtifacts)

(fn GetRandomFilteredCards
  (params (Amount :type Integer) (PossibleTags :type Gameplay%20Tag%20Container%20Structure) (RequiredTags :type Gameplay%20Tag%20Container%20Structure) (bExactMatch :type Boolean))
  (bind _randomcards (CallFunction|GetRandomCardsbyTagWeights (LocalVariables|GetLocalEmptyWeights) PossibleTags RequiredTags bExactMatch Amount))
  (return _randomcards))