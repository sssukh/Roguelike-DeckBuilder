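; BP_TurnManagerRLDB is a turn manager that provides helpers for ordering actors by initiative within a round.
; It inserts actors into an initiative array in descending order and finds the fastest valid actor in RoundOrderActors, reading initiative through GetInitiativeMessage.
; It also checks all BP_Minion actors for a living one with an exact gameplay tag.
; The minion-by-ID lookup, friendly name and priority functions are empty stubs.
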(fn ConstructionScript)

(fn AddActortoInitiative
  (params (Actor :type Actor%20Object%20Reference) (InitativeArray :type Array%20of%20Actor%20Object%20References))
  (for (_array_element _array_index) InitativeArray
    (bind _initiative (Class|BPIInitiativeRLDB|GetInitiative(Message) _array_element))
    (bind _initiative_2 (Class|BPIInitiativeRLDB|GetInitiative(Message) Actor))
    (if (>= _initiative_2 _initiative)
      (Utilities|Array|Insert InitativeArray Actor _array_index)
      (return _array_index)))
  (Utilities|Array|Add InitativeArray Actor)
  (return 0))

(fn CheckforRemainingMinionswithTag
  (params (Tag :type Gameplay%20Tag%20Structure))
  (bind _outactors (Actor|GetAllActorsOfClass "/Game/RLDB/Blueprints/Core/BP_Minion.BP_Minion_C"))
  (for _array_element _outactors
    (if (and (GameplayTags|HasTag (Default|GetGameplayTags _array_element) Tag true) (not (Variables|/Game/RLDB/Blueprints/Core/BP_Minion.BP_Minion_C|GetbDead _array_element)))
      (return true)))
  (return false))

(fn GetRemainingActorwithHighestInitiative
  (for _array_element (Variables|Default|GetRoundOrderActors)
    (bind _initiative (Class|BPIInitiativeRLDB|GetInitiative(Message) _array_element))
    (if (> _initiative (LocalVariables|GetLocalInitiative))
      (LocalVariables|SetLocalInitiative _initiative)
      (LocalVariables|SetLocalFastestActor _array_element)))
  (return (Utilities|IsValid (LocalVariables|GetLocalFastestActor)) (LocalVariables|GetLocalFastestActor)))

(fn FindMinionAmongRemaining
  (params (MinionUniqueId :type String)))

(fn GetFriendlyName
  (return ""))

(fn GetPriority
  (return 0.0))