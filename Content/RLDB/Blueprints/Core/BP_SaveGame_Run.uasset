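; BP_SaveGame_Run is a save game Blueprint that holds the persistent state of a run in what appears to be a deck-building game with node maps.
; Its single SavePersistentData function copies the passed-in heroes, deck, artifacts, map progress, level, current encounter, reward settings and completed story encounters into member variables.
; It only stores the data, with no disk write or load logic in this graph.
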(fn SavePersistentData
  (params (PersistentHeroes :type Array%20of%20DELETE%20F%20Minion%20Structures) (Deck :type Array%20of%20F%20Card%20Structures) (VisitedNodes :type Array%20of%20Integers) (Artifacts :type Array%20of%20F%20Status%20Structures) (LevelName :type String) (CurrentEncounter :type F%20Encounter%20Structure) (CurrentNodeMap :type String) (RewardTables :type Array%20of%20Data%20Table%20Object%20References) (AllowedCardRewardTags :type Gameplay%20Tag%20Container%20Structure) (DoneStoryEncounters :type Array%20of%20Data%20Table%20Row%20Handle%20Structures))
  (Variables|Default|SetPersistentHeroes PersistentHeroes)
  (Variables|Default|SetDeck Deck)
  (Variables|Default|SetVisitedNodes VisitedNodes)
  (Variables|Default|SetArtifacts Artifacts)
  (Variables|Default|SetLevelName LevelName)
  (Variables|Default|SetCurrentEncounter CurrentEncounter)
  (Variables|Default|SetCurrentNodeMap CurrentNodeMap)
  (Variables|Default|SetRewardTables RewardTables)
  (Variables|Default|SetAllowedCardRewardTags AllowedCardRewardTags)
  (Variables|Default|SetDoneStoryEncounters DoneStoryEncounters)
  (return))