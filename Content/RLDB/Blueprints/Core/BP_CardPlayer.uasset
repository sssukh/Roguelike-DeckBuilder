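; BP_CardPlayer is the card player actor of the RLDB card game, owning card piles, handling menu/mouse input and relaying messages to PlayerUI.
; On BeginPlay it maps piles by tag, binds dispatcher-hub events and applies artifact statuses from the game instance.
; Turn starts queue a new-player-turn action, while Hero deaths purge that hero's cards from draw, discard and hand.
; Statuses are components created on demand; PlayerUI creation is disconnected.
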(event Custom|DisplayScreenLogMessage
  (params (Message :type Text) (Color :type Linear%20Color%20Structure :default "(R=1.000000,G=0.000000,B=0.000000,A=1.000000)"))
  (Default|DisplayScreenLogMessage (Variables|Default|GetPlayerUI) Message Color))

(event Input|EnhancedActionEvents|EnhancedInputActionIA_Menu
  (params (ActionValue :type Boolean) (ElapsedSeconds :type Float%20%28double-precision%29) (TriggeredSeconds :type Float%20%28double-precision%29) (InputAction :type Input%20Action%20Object%20Reference :default "/Game/RLDB/Input/IA_Menu.IA_Menu"))
  (:Started
    (Default|ToggleinGameMenu (Variables|Default|GetPlayerUI)) ; Note. Input ideally handled from Player Controller or Pawn and set in Input Config.\nIt is handled here to allow for easier project migration, but for your final project, consider moving
  ))

(event EventRunEvent
  (params (EventTag :type Gameplay%20Tag%20Structure) (CallingObject :type Object%20Object%20Reference%20%28by%20ref%29) (bGlobal :type Boolean) (Payload :type Object%20Object%20Reference%20%28by%20ref%29) (CallTags :type Gameplay%20Tag%20Container%20Structure%20%28by%20ref%29))
  (if (not bGlobal)
    (|SwitchGameplayTag EventTag
      (:Event.TurnStart
        (CallFunction|QueueEventinGlobalDispatcherHub "(TagName=\"Event.Action.NewPlayerTurn\")" self 0 -1.0)))
    (else
      (|SwitchGameplayTag EventTag
        (:Event.Death
          (bind _asactor (Utilities|Casting|CastToActor CallingObject))
          (if (Utilities|IsValid (Actor|GetComponentbyClass _asactor "/Game/RLDB/Blueprints/Core/BP_GameplayTagComponent.BP_GameplayTagComponent_C"))
            (if (GameplayTags|HasTag (Variables|/Game/RLDB/Blueprints/Core/BP_GameplayTagComponent.BP_GameplayTagComponent_C|GetGameplayTags (Actor|GetComponentbyClass _asactor "/Game/RLDB/Blueprints/Core/BP_GameplayTagComponent.BP_GameplayTagComponent_C")) "(TagName=\"Target.Hero\")" true)
              (Default|RemoveAllCardsOwnedbyActor (Variables|Default|GetBP_PileComponent_Draw) _asactor))))))))

(event EventInitializeStoryEncounter
  (params (EncounterData :type Data%20Table%20Row%20Handle%20Structure) (bIsFirstScreen :type Boolean))
  (Default|InitializeStoryEncounter (Variables|Default|GetPlayerUI) EncounterData bIsFirstScreen))

(event EventBeginPlay
  (Input|AddMappingContext (PlayerController|LocalPlayerSubsystems|GetEnhancedInputLocalPlayerSubsystem (Game|GetPlayerController 0)) "/Game/RLDB/Input/IMC_RLDB.IMC_RLDB" 0 "(bIgnoreAllPressedKeysUntilRelease=True,bForceImmediately=False,bNotifyUserSettings=False)")
  (CallFunction|GeneratePileTagLookup)
  (Default|BindEventtoHub (Variables|Default|GetBP_DispatcherHubComponent_Local) self "(TagName=\"Event.TurnStart\")")
  (CallFunction|BindEventtoGlobalDispatcherHub self "(TagName=\"Event.Death\")")
  (bind _artifacts (Class|BPICardGameInstance|GetArtifactsfromInstance(Message) (Game|GetGameInstance)))
  (for _array_element _artifacts
    (CallFunction|AddtoStatus (.StatusClass (Utilities|Struct|BreakFStatus _array_element)) (.Value (Utilities|Struct|BreakFStatus _array_element)) false self))
  (Variables|/Script/Engine.PlayerController|SetbShowMouseCursor (Game|GetPlayerController 0) true))

(event Input|MouseEvents|LeftMouseButton
  (params (Key :type Key%20Structure :default "None"))
  (:Released
    (CallFunction|CallEventwithCallTagsinGlobalDispatcherHub "(TagName=\"Event.MouseRelease\")" self 0 "(GameplayTags=((TagName=\"Flag.Active\")))")))

(event Input|MouseEvents|RightMouseButton
  (params (Key :type Key%20Structure :default "None"))
  ;[0.7448 0.5161 0 1 10] v1.4
  (:Released
    (CallFunction|CallEventwithCallTagsinGlobalDispatcherHub "(TagName=\"Event.MouseRelease\")" self 0 "(GameplayTags=)")))

(fn ConstructionScript)

(fn GetPilewithPileTag
  (params (PileTag :type Gameplay%20Tag%20Structure))
  (bind _piletaglookup (Variables|Default|GetPileTagLookup))
  (bind (_value _returnvalue) (Utilities|Map|Find _piletaglookup PileTag))
  (return _returnvalue _value))

(fn GeneratePileTagLookup
  (for _array_element (Actor|GetComponentsByClass "/Game/RLDB/Blueprints/Piles/BP_PileComponent.BP_PileComponent_C")
    (Utilities|Map|Add (Variables|Default|GetPileTagLookup) (Variables|/Game/RLDB/Blueprints/Piles/BP_PileComponent.BP_PileComponent_C|GetPileTag _array_element) _array_element))
  (return))

(fn AddtoStatus
  (params (StatusClass :type BP%20Status%20Class%20Reference) (Amount :type Integer) (bShowSplash :type Boolean) (Payload :type Object%20Object%20Reference))
  (bind _returnvalue (Actor|GetComponentbyClass StatusClass))
  (Utilities|IsValid _returnvalue
    (:Is%20Valid
      (bind _newvalue (Default|AddStatusValue _returnvalue Amount false false false Payload))
      (return _newvalue))
    (:Is%20Not%20Valid
      (if (or (> Amount 0) (Utilities|GetClassDefaults StatusClass))
        (bind _returnvalue_2 (Game|AddComponentbyClass StatusClass 0 (Variables|Default|GetPlayerUI)))
        (Default|AddStatusValue _returnvalue_2 Amount false false true Payload)
        (return Amount)
        (else
          (return 0))))))

(fn AttemptMarkTarget
  (params (ValidTargets :type Gameplay%20Tag%20Container%20Structure))
  (return false))

(fn CheckifValidTarget
  (params (ValidTargets :type Gameplay%20Tag%20Container%20Structure))
  (return (GameplayTags|HasTag ValidTargets "(TagName=\"Target.CardPlayer\")" true)))

(fn GetFriendlyName
  (return "Card Player"))

(fn GetInitiative
  (return (Math|Conversions|ToFloat(Integer) (Variables|/Game/RLDB/Blueprints/Statuses/BP_Status.BP_Status_C|GetStatusValue (Variables|Default|GetBP_Status_Initiative)))))

(fn GetMinionUniqueId
  (return ""))

(fn GetPriority
  (return (Math|Conversions|ToFloat(Integer) (Variables|/Game/RLDB/Blueprints/Statuses/BP_Status.BP_Status_C|GetStatusValue (Variables|Default|GetBP_Status_Initiative)))))

(fn GetPuppet
  (return 0))

(fn GetStatusMax
  (params (Status :type BP%20Status%20Class%20Reference))
  (return false 0))

(fn GetStatusValue
  (params (Status :type BP%20Status%20Class%20Reference))
  (bind _returnvalue (Actor|GetComponentbyClass Status))
  (if (Utilities|IsValid _returnvalue)
    (return true (Variables|/Game/RLDB/Blueprints/Statuses/BP_Status.BP_Status_C|GetStatusValue _returnvalue))
    (else
      (return false 0))))

(fn MarkTarget
  (return true))

(fn SetStatusMax
  (params (Status :type BP%20Status%20Class%20Reference) (NewMax :type Integer))
  (return false))

(fn SubtractfromStatus
  (params (StatusClass :type BP%20Status%20Class%20Reference) (Amount :type Integer) (bShowSplash :type Boolean) (Payload :type Object%20Object%20Reference))
  (bind _newvalue (CallFunction|AddtoStatus StatusClass (* Amount -1) true Payload))
  (return _newvalue))