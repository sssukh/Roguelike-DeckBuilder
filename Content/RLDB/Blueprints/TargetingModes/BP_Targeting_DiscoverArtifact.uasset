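; Card-effect targeting mode that rolls a random artifact and offers it to the player on a reward screen.
; Rarity weights come from the effect's data row, falling back to the Normal row of DT_RarityWeights, and previews find no targets.
; The artifact lives as a component on a temporary actor until the screen returns.
; Unless skipped, it becomes a player status, then targeting completes and the game saves.
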(event Custom|ValidateAndTransferArtifact
  (params (bSkipped :type Boolean) (Artifact :type BP%20Status%20Object%20Reference))
  (EventDispatchers|UnbindEventfromOnReturnSelection (stale Custom|BindToArtifactConfirm CardRewardScreen) (delegate Custom|ValidateAndTransferArtifact))
  (if bSkipped
    _
    (else
      (bind _cardplayer (CallFunction|GetCardPlayer))
      (Default|AddtoStatus _cardplayer (Utilities|GetClass Artifact) (Variables|/Game/RLDB/Blueprints/Statuses/BP_Status.BP_Status_C|GetStatusValue Artifact) true)))
  (Actor|DestroyActor (Variables|Default|GetTempArtifactHolder))
  (Default|CallOnInputTargetsReceived (Utilities|Array|MakeArray 0))
  (Class|DELETEBPICardGameInstance|AttemptSaveGame(Message) (Game|GetGameInstance) "" false))

(event Custom|BindToArtifactConfirm
  (params (CardRewardScreen :type WBP%20Artifact%20Reward%20Screen%20Object%20Reference))
  (EventDispatchers|BindEventtoOnReturnSelection CardRewardScreen (delegate Custom|ValidateAndTransferArtifact)))

(fn FindValidTargets
  (params (SpecifiedTargets :type Array%20of%20Actor%20Object%20References) (CardEffect :type F%20Card%20Effect%20Structure) (Card :type BP%20Card%20Object%20Reference) (bPreview :type Boolean))
  (bind _useddata (CallFunction|GetEffectUsedData CardEffect))
  (if bPreview
    (return false 0)
    (else
      (if (Utilities|IsValid (.datatable _useddata))
        (bind _returnvalue (Utilities|GetDataTableRow (.datatable _useddata) (.rowname _useddata))
          (:then
            (LocalVariables|SetLocalRarityWeights (Utilities|Struct|BreakFRarityWeights _returnvalue)))
          (:RowNotFound
            (bind _returnvalue_2 (Utilities|GetDataTableRow "/Game/RLDB/Data/DT_RarityWeights.DT_RarityWeights" "Normal" :!label _label)
              (:then
                (LocalVariables|SetLocalRarityWeights (.rarityweights _returnvalue_2)))
              (:RowNotFound
                (return false 0)))))
        (else
          (goto _label)))
      (bind _cardplayer (CallFunction|GetCardPlayer))
      (bind (_bsuccess _pickedartifacts) (Default|GetRandomArtifactsbyCustomTagWeights (Variables|/Game/RLDB/Blueprints/Core/BP_CardPlayer.BP_CardPlayer_C|GetBP_ChanceManagerComponent _cardplayer) (LocalVariables|GetLocalRarityWeights) 1 true))
      (if _bsuccess
        (Variables|Default|SetPickedArtifact (Utilities|Array|Get(acopy) _pickedartifacts))
        (bind _returnvalue_3 (Game|SpawnActorfromClass "/Script/Engine.Actor" (Math|Transform|MakeTransform "0, 0, 0" "0, 0, 0" "1.000000,1.000000,1.000000") "Undefined" "OverrideRootScale" 0 0))
        (bind _output_get (Variables|Default|SetTempArtifactHolder _returnvalue_3))
        (bind _returnvalue_4 (Game|AddComponentbyClass _output_get (.StatusClass (Utilities|Struct|BreakFStatus (Variables|Default|GetPickedArtifact))) (.Value (Utilities|Struct|BreakFStatus (Variables|Default|GetPickedArtifact))) 0 true (.GameplayTags (Utilities|Struct|BreakFStatus (Variables|Default|GetPickedArtifact)))))
        (Game|SpawnActorfromClass "/Game/RLDB/Blueprints/CardActions/BP_Action_ArtifactRewardScreen.BP_Action_ArtifactRewardScreen_C" (Math|Transform|MakeTransform "0, 0, 0" "0, 0, 0" "1.000000,1.000000,1.000000") "Undefined" "OverrideRootScale" 0 _returnvalue_4 -1.0 0)
        (bind _returnvalue_5 (Actor|GetActorOfClass "/Game/RLDB/Blueprints/Core/BP_CardPlayer.BP_CardPlayer_C"))
        (CallFunction|BindtoArtifactConfirm (Variables|/Game/RLDB/Widgets/WBP_Layout_RLDB.WBP_Layout_RLDB_C|GetWBP_ArtifactReward (Variables|/Game/RLDB/Blueprints/Core/BP_CardPlayer.BP_CardPlayer_C|GetPlayerUI _returnvalue_5)))
        (return true 0)
        (else
          (return false 0))))))