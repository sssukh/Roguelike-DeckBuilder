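; BP_Status_Card_ManaModifier is a card status, named for modifying mana, that attaches to a BP_Card.
; On BeginPlay it caches its owning card and binds itself to that card's local exit-hand event.
; RunEvent filters for calls from the owning card and switches on the event tag, but no response is wired, and this graph contains no mana-changing logic.
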(event EventBeginPlay
  (|CallParentFunction)
  (bind _asbp_card (Utilities|Casting|CastToBP_Card (Components|GetOwner)))
  (bind _output_get (Variables|Default|SetOwningCard _asbp_card))
  (Default|BindLocalCardEvents _output_get self "(GameplayTags=((TagName=\"Event.Card.ExitHand\"),(TagName=\"Event.Card.ModifyInHand\")))"))

(event EventRunEvent
  (params (EventTag :type Gameplay%20Tag%20Structure) (CallingObject :type Object%20Object%20Reference%20%28by%20ref%29) (bGlobal :type Boolean) (Payload :type Object%20Object%20Reference%20%28by%20ref%29) (CallTags :type Gameplay%20Tag%20Container%20Structure%20%28by%20ref%29))
  (if (== CallingObject (Variables|Default|GetOwningCard))
    (|SwitchGameplayTag EventTag)))