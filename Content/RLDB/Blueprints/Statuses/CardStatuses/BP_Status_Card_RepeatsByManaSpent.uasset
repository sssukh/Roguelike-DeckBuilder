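; BP_Status_Card_RepeatsByManaSpent is a card status that makes its owning card cost and repeat according to a given Mana value.
; UpdateFromMana sets the card's Mana stat cost to that value, clamped to at least one, and sets its repetitions to one less than that.
; It then notifies the card that it has been modified.
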(fn UpdatefromMana
  (params (Mana :type Integer))
  (Default|SetUseRuleCost (Variables|Default|GetOwningCard) "/Game/RLDB/Blueprints/CardUseRules/BP_UseRule_StatCost.BP_UseRule_StatCost_C" "/Game/RLDB/Blueprints/Statuses/BP_Status_Mana.BP_Status_Mana_C" (Math|Integer|Max(Integer) Mana 1) "NewEnumerator0" true)
  (Default|SetCardRepetitions (Variables|Default|GetOwningCard) "NewEnumerator0" (- (Math|Integer|Max(Integer) Mana 1) 1))
  (Default|CallOnThisCardModified (Variables|Default|GetOwningCard))
  (return))