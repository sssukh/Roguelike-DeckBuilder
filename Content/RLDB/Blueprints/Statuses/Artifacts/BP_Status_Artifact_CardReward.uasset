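; Artifact status that stores the data row handle for a card reward, judging by its name and variables.
; When value is added, it runs the parent logic, then fills an unset reward handle from the BP_CardEffect payload's UsedData, falling back to DefaultRewardData if that data is invalid.
; Once the handle has a valid table, later additions leave it unchanged.
; The Interact override has no connected logic.
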(fn Interact
  (params (Tags :type Gameplay%20Tag%20Container%20Structure)))

(fn AddStatusValue
  (params (Amount :type Integer) (bShowSplashNumber :type Boolean) (bShowSplashIcon :type Boolean) (bRefreshAppearance :type Boolean) (Payload :type Object%20Object%20Reference))
  (bind _newvalue (|CallParentFunction Amount bShowSplashNumber bShowSplashIcon bRefreshAppearance Payload))
  (if (not (Utilities|IsValid (.datatable (Variables|Default|GetCardRewardData))))
    (bind _asbp_card_effect (Utilities|Casting|CastToBP_CardEffect Payload)
      (:then
        (Variables|Default|SetCardRewardData (select (Utilities|IsValid (.DataTable (Utilities|Struct|BreakDataTableRowHandle (Variables|/Game/RLDB/Blueprints/CardEffects/BP_CardEffect.BP_CardEffect_C|GetUsedData _asbp_card_effect)))) (Variables|/Game/RLDB/Blueprints/CardEffects/BP_CardEffect.BP_CardEffect_C|GetUsedData _asbp_card_effect) (Variables|Default|GetDefaultRewardData)))
        (return _newvalue))
      (:CastFailed
        _)))
  (return _newvalue))