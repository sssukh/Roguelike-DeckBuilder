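; Artifact status for card combat that records artifacts gained by the card player in the game instance.
; AddStatusValue sends class, amount and tags to the game instance, then runs the parent logic.
; When the player passes itself as payload while restoring artifacts at combat start, recording is skipped to avoid duplication.
; BeginPlay skips parent initialization on minion owners, and Interact is empty.
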(event EventBeginPlay
  (Utilities|Casting|CastToBP_CardPlayer (Components|GetOwner)
    (:then
      (|CallParentFunction))
    (:CastFailed
      (bind _asbp_minion (Utilities|Casting|CastToBP_Minion (Components|GetOwner))
        (:then
          (if (GameplayTags|HasTag (Default|GetGameplayTags _asbp_minion) "(TagName=\"Target.Hero\")" true)
            _))
        (:CastFailed
          (|CallParentFunction))))))

(fn Interact
  (params (Tags :type Gameplay%20Tag%20Container%20Structure)))

(fn AddStatusValue
  (params (Amount :type Integer) (bShowSplashNumber :type Boolean) (bShowSplashIcon :type Boolean) (bRefreshAppearance :type Boolean) (Payload :type Object%20Object%20Reference))
  (bind _asbp_card_player (Utilities|Casting|CastToBP_CardPlayer (Components|GetOwner))
    (:then
      (if (!= _asbp_card_player Payload) ; When the Card Player adds artifacts from the gam instance\nat the start of combat it passes itelf through as a payload.\nSignals that this should not be added again to the instance,\nas this would duplicate its value.
        (Class|DELETEBPICardGameInstance|AddArtifacttoInstance(Message) (Game|GetGameInstance) (Utilities|Struct|MakeFStatus (Utilities|GetClass self) Amount (Variables|Default|GetGameplayTags)))
        (bind _newvalue (|CallParentFunction Amount bShowSplashNumber bShowSplashIcon bRefreshAppearance Payload))
        (return _newvalue)
        (else
          _)))
    (:CastFailed
      _))
  (bind _newvalue_2 (|CallParentFunction Amount bShowSplashNumber bShowSplashIcon bRefreshAppearance Payload))
  (return _newvalue_2))