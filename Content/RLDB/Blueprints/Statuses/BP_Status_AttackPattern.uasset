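; Attack pattern status in a card game that takes its look and tooltips from a card, with NextCard as the reference for its appearance.
; HasAppearanceChanged reports whether NextCard's portrait, frame tint or repetition count differs from the stored icon, tint and last repetition count.
; UpdateTooltipsFromCard replaces the status tooltips with a list built from the given card's tooltips, each paired with a false flag.
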(fn HasAppearanceChanged
  (bind _nextcard (Variables|Default|GetNextCard))
  (return (Math|Boolean|ORBoolean (!= (Variables|Default|GetIcon) (Default|GetCardPortrait _nextcard "NewEnumerator2")) (!= (.specifiedcolor (Default|GetCardFrameTint _nextcard "NewEnumerator2")) (Variables|Default|GetTint)) (!= (Default|GetCardRepetitions _nextcard "NewEnumerator0") (Variables|Default|GetLastCardRepetitions)))))

(fn UpdateTooltipsfromCard
  (params (Card :type BP%20Card%20Object%20Reference))
  (for _array_element (Default|GetCardTooltips Card "NewEnumerator0")
    (Utilities|Array|Add (LocalVariables|GetLocalTooltips) (Utilities|Struct|Make _array_element false)))
  (Variables|Default|SetTooltips (LocalVariables|GetLocalTooltips))
  (return))