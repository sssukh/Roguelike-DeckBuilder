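; BP_Action_LoadMap is a card action that opens the level named by its Level variable.
; PlayAction creates a WBP_ScreenFade widget, adds it to the viewport and plays its Occlude animation.
; A delay sized to that animation's end time, plus a small margin, holds the level load until the fade has finished.
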(event EventPlayAction
  ;[0 0 0] Loads an input level on queue
  (bind _returnvalue (UserInterface|CreateWidget "/Game/CrownOfSin/Widgets/WBP_ScreenFade.WBP_ScreenFade_C"))
  (UserInterface|Viewport|AddtoViewport _returnvalue 0)
  (UserInterface|Animation|PlayAnimation _returnvalue (Variables|/Game/CrownOfSin/Widgets/WBP_ScreenFade.WBP_ScreenFade_C|GetOcclude _returnvalue) 0.0 1 "Forward" 1.0 false)
  (Utilities|FlowControl|Delay (+ (Class|WidgetAnimation|GetEndTime (Variables|/Game/CrownOfSin/Widgets/WBP_ScreenFade.WBP_ScreenFade_C|GetOcclude _returnvalue)) 0.01))
  (Game|OpenLevel(byName) (Utilities|String|StringToName (Variables|Default|GetLevel))))

(fn ConstructionScript
  (|CallParentFunction))