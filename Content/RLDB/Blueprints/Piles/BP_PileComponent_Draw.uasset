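; BP_PileComponent_Draw is the draw pile component of a card game, able to refill itself from the discard pile.
; ReshuffleDiscardIntoDraw finds the sibling discard pile component on the same owner and acts only if it holds cards.
; It fires the Event.Reshuffle tag through the global dispatcher hub, then passes the discard cards to AssignExistingCards and clears the discard pile.
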(fn ReshuffleDiscardIntoDraw
  (bind _returnvalue (Components|GetOwner))
  (bind _returnvalue_2 (Actor|GetComponentbyClass _returnvalue "/Game/RLDB/Blueprints/Piles/BP_PileComponent_Discard.BP_PileComponent_Discard_C"))
  (bind _cards (Variables|/Game/RLDB/Blueprints/Piles/BP_PileComponent.BP_PileComponent_C|GetCards _returnvalue_2))
  (if (> (Utilities|Array|Length _cards) 0)
    (Class|FunctionLibraryEvent|CallEventinGlobalDispatcherHub "(TagName=\"Event.Reshuffle\")" self 0)
    (CallFunction|AssignExistingCards _cards)
    (Utilities|Array|Clear _cards)
    (return)
    (else
      (return))))