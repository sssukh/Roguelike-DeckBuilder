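; Card use rule Blueprint meant to gate playing a card on a stat cost.
; CheckIfUseAllowed holds logic that looks up the status component class from UseRuleData, compares its value to the cost, and builds a "Not Enough" message with the stat's name.
; That logic is disconnected from the function entry, so it never runs.
; ResolveUseConsequence is also a stub: it deducts nothing, and its return of true is unconnected.
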(event EventBeginPlay
  (|CallParentFunction) ; This node is disabled and will not be called.\nDrag off pins to build functionality.
)

(event EventTick
  (params (DeltaSeconds :type Float%20%28single-precision%29))
  (|CallParentFunction DeltaSeconds) ; This node is disabled and will not be called.\nDrag off pins to build functionality.
)

(fn CheckifUseAllowed
  (params (UseRuleData :type F%20Use%20Rule%20Structure)))

(fn ResolveUseConsequence
  (params (UseRuleData :type F%20Use%20Rule%20Structure)))