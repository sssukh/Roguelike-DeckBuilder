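; Card use rule that lets a card be used only if its owner has enough of a given status to cover a cost.
; CheckIfUseAllowed finds the owner's component of the rule data's Status class and compares its StatusValue to the Cost.
; A shortfall returns a "Not Enough" message with the status's friendly name, while a missing component fails silently.
; ResolveUseConsequence is a stub, so this rule does not deduct the cost.
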(event EventBeginPlay
  (|CallParentFunction) ; This node is disabled and will not be called.\nDrag off pins to build functionality.
)

(event EventTick
  (params (DeltaSeconds :type Float%20%28single-precision%29))
  (|CallParentFunction DeltaSeconds) ; This node is disabled and will not be called.\nDrag off pins to build functionality.
)

(fn CheckifUseAllowed
  (params (UseRuleData :type F%20Use%20Rule%20Structure))
  (bind (_status _cost) (Utilities|Struct|BreakFUseRule UseRuleData))
  (bind _parentcard (Variables|Default|GetParentCard))
  (bind _returnvalue (Components|GetOwner _parentcard))
  (bind _returnvalue_2 (Actor|GetComponentbyClass _returnvalue _status))
  (if (Utilities|IsValid _returnvalue_2)
    (if (>= (Variables|/Game/RLDB/Blueprints/Statuses/BP_Status.BP_Status_C|GetStatusValue _returnvalue_2) _cost)
      (return true "")
      (else
        (return false (Utilities|String|Append "Not Enough " (Utilities|String|ToString(Text) (Variables|/Game/RLDB/Blueprints/Statuses/BP_Status.BP_Status_C|GetFriendlyName _returnvalue_2))))))
    (else
      (return false ""))))

(fn ResolveUseConsequence
  (params (UseRuleData :type F%20Use%20Rule%20Structure)))