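; DELETE_BP_MapEvent_Multi is a node-map event, prefixed DELETE, that dispatches to another map event component.
; RunMapEvent looks up the event's data table row, then reuses or adds a component of the row's MapEventClass on the owner.
; It casts that to DELETE_BP_MapEventComponent and runs the row's SpecificEvent, falling back to ChooseRandomEncounter when that row does not exist.
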(event EventRunMapEvent
  (params (EventData :type Data%20Table%20Row%20Handle%20Structure))
  (bind _returnvalue (Utilities|GetDataTableRow (.datatable EventData) (.rowname EventData))
    (:then
      (Variables|Default|SetCurrentMapEventStruct _returnvalue)
      (if (Utilities|IsValid (Actor|GetComponentbyClass (Components|GetOwner) (Utilities|Struct|BreakFMapEvent _returnvalue)))
        (Variables|Default|SetCurrentMapEventComponent (Actor|GetComponentbyClass (Components|GetOwner) (Utilities|Struct|BreakFMapEvent _returnvalue)))
        (else
          (bind _returnvalue_2 (Game|AddComponentbyClass (Components|GetOwner) (Utilities|Struct|BreakFMapEvent _returnvalue)))
          (Variables|Default|SetCurrentMapEventComponent _returnvalue_2)))
      (bind _asdelete_bp_map_event_component (Utilities|Casting|CastToDELETE_BP_MapEventComponent (Variables|Default|GetCurrentMapEventComponent)))
      (bind _returnvalue_3 (Class|DataTableFunctionLibrary|DoesDataTableRowExist (.DataTable (Utilities|Struct|BreakDataTableRowHandle (Utilities|Struct|BreakFMapEvent (Variables|Default|GetCurrentMapEventStruct)))) (.RowName (Utilities|Struct|BreakDataTableRowHandle (Utilities|Struct|BreakFMapEvent (Variables|Default|GetCurrentMapEventStruct))))))
      (if _returnvalue_3
        (Default|RunMapEvent _asdelete_bp_map_event_component (Utilities|Struct|BreakFMapEvent (Variables|Default|GetCurrentMapEventStruct)))
        (else
          (bind _randomencounter (Default|ChooseRandomEncounter _asdelete_bp_map_event_component (Variables|Default|GetCurrentMapEventStruct)))
          (Default|RunMapEvent _asdelete_bp_map_event_component (Utilities|Struct|MakeDataTableRowHandle (.datatable _randomencounter) (.rowname _randomencounter))))))))