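; Node-map event for Arena encounters, named with a DELETE prefix, that launches an encounter's level from a data table row.
; RunMapEvent plays a screen fade, waits out the animation, then saves the game, stores the current encounter and marks it done on the game instance before opening the row's level.
; GetEncounterTags returns the gameplay tags of a given encounter row.
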(event EventRunMapEvent
  (params (EventData :type Data%20Table%20Row%20Handle%20Structure))
  (bind (_datatable _rowname) (Utilities|Struct|BreakDataTableRowHandle EventData))
  (bind _returnvalue (UserInterface|CreateWidget "/Game/CrownOfSin/Widgets/WBP_ScreenFade.WBP_ScreenFade_C"))
  (UserInterface|Viewport|AddtoViewport _returnvalue 0)
  (UserInterface|Animation|PlayAnimation _returnvalue (Variables|/Game/CrownOfSin/Widgets/WBP_ScreenFade.WBP_ScreenFade_C|GetOcclude _returnvalue) 0.0 1 "Forward" 1.0 false)
  (Utilities|FlowControl|Delay (+ (Class|WidgetAnimation|GetEndTime (Variables|/Game/CrownOfSin/Widgets/WBP_ScreenFade.WBP_ScreenFade_C|GetOcclude _returnvalue)) 0.01))
  (bind _returnvalue_2 (Utilities|GetDataTableRow _datatable _rowname)
    (:then
      (Class|DELETEBPICardGameInstance|AttemptSaveGame(Message) (Game|GetGameInstance) "" true)
      (Class|DELETEBPICardGameInstance|SetCurrentEncounterinInstance(Message) (Game|GetGameInstance) _returnvalue_2)
      (Class|DELETEBPICardGameInstance|AddDoneStoryEncountertoInstance(Message) (Game|GetGameInstance) EventData)
      (Game|OpenLevel(byName) (Utilities|String|StringToName (Utilities|Struct|BreakFEncounter _returnvalue_2))))))

(fn GetEncounterTags
  (params (DataTable :type Data%20Table%20Object%20Reference) (RowName :type Name :default "None"))
  (bind _returnvalue (Utilities|GetDataTableRow DataTable RowName)
    (:then
      (return (Utilities|Struct|BreakFEncounter _returnvalue)))
    (:RowNotFound
      (return ""))))