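; Map event Blueprint for story encounters on the node map, marked DELETE in its asset name.
; RunMapEvent records encounters that have a valid DataTable as done through the game instance, then initializes the card player's story encounter on its first screen.
; Without a valid table, it starts FillerEncounter instead and records nothing.
; A helper function looks up an encounter's GameplayTags by DataTable row.
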(event EventRunMapEvent
  (params (EventData :type Data%20Table%20Row%20Handle%20Structure))
  (Utilities|IsValid (.DataTable (Utilities|Struct|BreakDataTableRowHandle EventData))
    (:Is%20Valid
      (Class|Object|AddDoneStoryEncountertoInstance(Message) (Game|GetGameInstance) EventData)
      (CallFunction|InitializeStoryEncounter (CallFunction|GetCardPlayerPure) EventData true))
    (:Is%20Not%20Valid
      (CallFunction|InitializeStoryEncounter (CallFunction|GetCardPlayerPure) (Variables|Default|GetFillerEncounter) true))))

(fn GetEncounterTags
  (params (DataTable :type Data%20Table%20Object%20Reference) (RowName :type Name :default "None"))
  (bind _returnvalue (Utilities|GetDataTableRow DataTable RowName)
    (:then
      (return (.GameplayTags (Utilities|Struct|BreakFStoryEncounter _returnvalue))))))