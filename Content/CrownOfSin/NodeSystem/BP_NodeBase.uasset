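; BP_NodeBase is a base Blueprint for node system nodes that signals to the player when a node can be clicked.
; Enable sets the Enabled flag, opens a gate and plays a timeline that scales NodeMesh in a wobble.
; The timeline re-enters the gate on finish to loop, until StopEnable clears the flag and closes the gate, letting the current wobble play out.
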(event EventEnable
  ;[0 0 0] Signals that node can be clicked and starts wobble animation to communicate this to the player
  (Variables|Default|SetbEnabled true)
  (Utilities|FlowControl|Sequence
    (:then_0
      (goto _label Open))
    (:then_1
      (bind _wobble (Timeline|TL_Wobble PlayFromStart)
        (:Update
          (Transformation|SetRelativeScale3D (Variables|Default|GetNodeMesh) (Math|Conversions|ToVector(Float) (+ 1.0 (* _wobble 0.2)))))
        (:Finished
          (Utilities|FlowControl|Gate true :!label _label
            (:Exit
              (Timeline|TL_Wobble PlayFromStart))))))))

(event EventStopEnable
  ;[0 0 0] Signals that node can be clicked and starts wobble animation to communicate this to the player
  (Variables|Default|SetbEnabled false)
  (Utilities|FlowControl|Gate true) ; enters at Close
)

(fn ConstructionScript)