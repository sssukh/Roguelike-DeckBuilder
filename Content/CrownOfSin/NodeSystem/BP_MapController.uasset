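; Player controller for the node map that creates the node map layout widget and handles mouse hover and clicking on nodes.
; Each tick it traces under the cursor and, when a new actor is hit, sends hover-off and hover-over messages, keeping HoveredActor if nothing is hit.
; A left press stores the hovered actor as ClickedNode, freezing hover changes.
; Release sends the click message if both still match, then clears ClickedNode.
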(event EventTick
  (params (DeltaSeconds :type Float%20%28single-precision%29))
  (bind _hitresult (Game|Player|GetHitResultUnderCursorbyChannel "TraceTypeQuery1" true))
  (bind _hitactor (Collision|BreakHitResult _hitresult))
  ;[0 0 0] Handle Node Map input
  (if (Utilities|IsValid _hitactor)
    (if (!= (Variables|Default|GetHoveredActor) _hitactor)
      (Variables|Default|GetClickedNode
        (:then)
        (:else
          (Class|InterfaceNode|HoverOffNode(Message) (Variables|Default|GetHoveredActor))
          (bind _output_get (Variables|Default|SetHoveredActor _hitactor))
          (Class|InterfaceNode|HoverOverNode(Message) _output_get))))))

(event EventBeginPlay
  (bind _returnvalue (UserInterface|CreateWidget "/Game/CrownOfSin/BluePrints/Widgets/NodeMap/WBP_NodeMapLayout.WBP_NodeMapLayout_C"))
  (UserInterface|Viewport|AddtoViewport _returnvalue 0))

(event Input|MouseEvents|LeftMouseButton
  (params (Key :type Key%20Structure))
  ;[0 0 0] Handle Node Map input
  (:Pressed
    (Variables|Default|SetClickedNode (Variables|Default|GetHoveredActor)))
  (:Released
    (if (== (Variables|Default|GetClickedNode) (Variables|Default|GetHoveredActor))
      (Class|InterfaceNode|ClickNode(Message) (Variables|Default|GetHoveredActor))
      (Variables|Default|SetClickedNode 0)
      (else
        (Variables|Default|SetClickedNode 0)))))

(fn ConstructionScript)