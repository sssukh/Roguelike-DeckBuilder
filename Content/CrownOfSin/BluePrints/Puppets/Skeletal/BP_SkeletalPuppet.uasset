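; Skeletal puppet actor Blueprint that handles fading the puppet in and out as it appears or disappears.
; One timeline, with play rate set by each event, drives the Opacity parameter on dynamic mesh materials and the bottom UI widget's render opacity.
; Disappearing plays it forward after a configurable delay, while appearing unhides the actor and plays it in reverse.
; The actor destroys itself when the timeline finishes at zero opacity.
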(event EventDisappearPuppet
  (params (InSpeedProp :type Float%20%28single-precision%29))
  (Components|Timeline|SetPlayRate (Variables|Default|GetTL_FadeOut) InSpeedProp)
  (Utilities|FlowControl|Delay (Variables|Default|GetDisappearFadeDelay))
  (bind _opacity (Timeline|TL_FadeOut PlayFromStart)
    (:Update
      (for _array_element (Variables|Default|GetDynamicMeshMaterials)
        (Rendering|Material|SetScalarParameterValue _array_element "Opacity" _opacity :!class /Script/Engine.MaterialInstanceDynamic)
        (Widget|SetRenderOpacity (UserInterface|GetWidget (Variables|Default|GetBottomUIWidgetComponent)) _opacity)))
    (:Finished
      (if (== _opacity 0.0)
        (Actor|DestroyActor)))))

(event EventAppearPuppet
  (params (InSpeedProp :type Float%20%28single-precision%29))
  (Components|Timeline|SetPlayRate (Variables|Default|GetTL_FadeOut) InSpeedProp)
  (Rendering|SetActorHiddenInGame false)
  (bind _opacity (Timeline|TL_FadeOut ReverseFromEnd)
    (:Update
      (for _array_element (Variables|Default|GetDynamicMeshMaterials)
        (Rendering|Material|SetScalarParameterValue _array_element "Opacity" _opacity :!class /Script/Engine.MaterialInstanceDynamic)
        (Widget|SetRenderOpacity (UserInterface|GetWidget (Variables|Default|GetBottomUIWidgetComponent)) _opacity)))
    (:Finished
      (if (== _opacity 0.0)
        (Actor|DestroyActor)))))

(fn ConstructionScript)