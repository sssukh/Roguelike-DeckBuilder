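; BP_MinionTrack manages a track of minions and animates their puppets sliding to their indexed track positions.
; SlideMinionstoPositions waits on a retriggerable delay, then snapshots the location of each entry in the Minions array.
; A timeline then lerps each minion's Puppet from that snapshot to the location GetTrackLocationAtIndex returns for its array index.
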(event EventSlideMinionstoPositions
  (params (InStartDelay :type Float%20%28single-precision%29))
  (Utilities|FlowControl|RetriggerableDelay InStartDelay)
  (Utilities|Array|Clear (Variables|Default|GetPuppetLocationsPreSlide))
  (for _array_element (Variables|Default|GetMinions)
    (Utilities|IsValid _array_element
      (:Is%20Valid
        (Utilities|Array|Add (Variables|Default|GetPuppetLocationsPreSlide) (Transformation|GetActorLocation _array_element)))
      (:Is%20Not%20Valid
        (Utilities|Array|Add :TargetArray (Variables|Default|GetPuppetLocationsPreSlide)))))
  (bind _slidescale (Timeline|SlidleTimeLine PlayFromStart)
    (:Update
      (for (_array_element_2 _array_index) (Variables|Default|GetMinions)
        (Transformation|SetActorLocation (Variables|/Script/CrownOfSin.MinionBase|GetPuppet _array_element_2) (Math|Vector|Lerp(Vector) (Utilities|Array|Get(acopy) (Variables|Default|GetPuppetLocationsPreSlide) _array_index) (Class|MinionTrack|GetTrackLocationatIndex _array_index false) _slidescale) false false)))))

(fn ConstructionScript)